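; Interactive button actor that cycles a sofa's material variants (blue, green, base layer) in a stereo viewer.
; OnBlur enables player input and shows the PresionaF prompt, OnDeblur reverses both, and each updates the text render.
; F or the motion controller right trigger advances a looping MultiGate.
; Its timelines drive SillonAzul and SillonVerde in a Material Parameter Collection, with the third disabling both to expose the base layer.
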(event `/Game/Blueprints/Btn1_Interface_BP.OnBlur`
  ;[1 1 1] Widget Contrls
  (`self.EnableInput` (`GameplayStatics.GetPlayerController` 0))
  (`SceneComponent.SetVisibility` (`self.Presiona F`) true false)
  (`TextRenderComponent.K2_SetText` (`self.TextRender`) (`self.blur`)))

(event `/Game/Blueprints/Btn1_Interface_BP.OnDeblur`
  ;[1 1 1] Widget Contrls
  (`self.DisableInput` (`GameplayStatics.GetPlayerController` 0))
  (`SceneComponent.SetVisibility` (`self.Presiona F`) false false)
  (`TextRenderComponent.K2_SetText` (`self.TextRender`) (`self.deblur`)))

(event `Key|MotionController_Right_Trigger`
  (params (Key :type "Key Structure"))
  ;[1 1 1] Change Parameter Collection Variable
  (:`Pressed`
    (`|MultiGate` false true :!label _label
      (:`Out 0`
        (bind (_direction _alpha) (`Timeline|Timeline_1` :!via `PlayFromStart`)
          (:`Update`
            ;;[1 1 1] Habilito sillon Azul
            (`KismetMaterialLibrary.SetScalarParameterValue` "/Game/Materials/Mat_StereoViewer_Collection.Mat_StereoViewer_Collection" "SillonAzul" _alpha))))
      (:`Out 1`
        (bind (_direction_2 _alpha_2) (`Timeline|Timeline_0` :!via `PlayFromStart`)
          (:`Update`
            ;;[1 1 1] Habilito sillon Verde
            (`KismetMaterialLibrary.SetScalarParameterValue` "/Game/Materials/Mat_StereoViewer_Collection.Mat_StereoViewer_Collection" "SillonVerde" _alpha_2))))
      (:`Out 2`
        (bind (_direction_3 _alpha_3 _newtrack_1) (`Timeline|Timeline_2` :!via `PlayFromStart`)
          (:`Update`
            ;;[1 1 1] Deshabilito los dos valores para obtener la capa inferior del material
            (`KismetMaterialLibrary.SetScalarParameterValue` "/Game/Materials/Mat_StereoViewer_Collection.Mat_StereoViewer_Collection" "SillonAzul" _newtrack_1)
            (`KismetMaterialLibrary.SetScalarParameterValue` "/Game/Materials/Mat_StereoViewer_Collection.Mat_StereoViewer_Collection" "SillonVerde" _newtrack_1)))))))

(event `Key|F`
  (params (Key :type "Key Structure"))
  ;[1 1 1] Change Parameter Collection Variable
  (:`Pressed`
    (goto _label)))

(fn `UserConstructionScript`)