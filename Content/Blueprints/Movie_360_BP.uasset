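; Debug Blueprint that exports a stereoscopic 360 panoramic screenshot of the level when T is pressed.
; The key press runs a chain of console commands that configure the Stereo Panoramic capture plugin (output folder, eye separation, slice angles, resolution, concurrency), then fire the screenshot.
; A panoramic movie export over a frame range and a sequence player start are present but unwired, so they never run.
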(event `Key|T`
  (params (Key :type "Key Structure"))
  (:`Pressed`
    (`KismetSystemLibrary.ExecuteConsoleCommand` "-usefixedtimestep -fps=60 -notexturestreaming")
    ;[1 1 1] Donde va a guardar las capturas
    (`KismetSystemLibrary.ExecuteConsoleCommand` "SP.OutputDir C:\\360")
    ;[1 1 1] Eye separation. Default=6.4f
    (`KismetSystemLibrary.ExecuteConsoleCommand` "SP.EyeSeparation 6.4f")
    ;[1 1 1] Cantidad de imagenes que saca para cada frame 360
    ; cuanto mas chicos son los paramentros>
    ; HorizontalAngularIncrement
    ; VerticalAngularIncrement
    ; mas imagenes saca por frame para armar el frame final 360
    ;
    ; (360 / HorizontalAngularIncrement) * (180 / VerticalAngularIncrement) * 2 (because it's per-eye)
    ;;[1 1 1] Angulo horizontal que gira para hacer cada captura del frame 360
    (`KismetSystemLibrary.ExecuteConsoleCommand` "SP.HorizontalAngularIncrement 2")
    ;;[1 1 1] Angulo vertical que gira para hacer cada captura del frame 360
    (`KismetSystemLibrary.ExecuteConsoleCommand` "SP.VerticalAngularIncrement 30")
    ;[1 1 1] FOV de las sub capturas
    (`KismetSystemLibrary.ExecuteConsoleCommand` "SP.CaptureHorizontalFOV 30")
    ;[1 1 1] Numero de capturas de estas partes del frame total simultaneas OJO puede sobrepasar la VRAM
    (`KismetSystemLibrary.ExecuteConsoleCommand` "SP.ConcurrentCaptures 6")
    ;[1 1 1] Me imagino que esto es para forzar el giro de la camara a 0 para que no salga el frame tumbado
    (`KismetSystemLibrary.ExecuteConsoleCommand` "SP.ShouldOverrideInitialYaw 0")
    ;[1 1 1] Finally, SP.CaptureSlicePixelWidth
    ; This value represents the size of 'each view' that you render (of the 2520 views you're going to be rendering per frame!), so reducing this can have an enormous impact on your overall rendering time. It's actually separate from your final output image and you should size it based on how many vertical 'steps' you're going to do (180/VerticalAngularIncrement), and how much multi-sampling you want for the final image.
    ;
    ; In effect, if your buffer was, say, 2048 and you have 6 vertical steps, then what you're really doing is rendering an image 12,288 pixels high. If your final output image is a 4096x2048 per-eye image then you can see that you really didn't NEED that many pixels in height to begin with; you've got enough for 6xFSAA there! We really only consider the vertical resolution here because, if you remember the image above, we're not even using the full width of the image, we're just grabbing the middle bit, so the width is less important here (it just has to be wide enough so that it has enough pixels to pull out of the middle).
    ;
    ; By contrast, if you set the value to 720 then you're now going to be rendering an effective height of ~4320 and downsampling that to 2048, STILL equivalent to 2xFSAA (which we've found is definitely good enough) and now your rendering times are going to be about 40 seconds for those 2520 views, instead of being about 3 minutes (it doesn't exactly scale linearly, but it's still a nice win).
    (`KismetSystemLibrary.ExecuteConsoleCommand` "SP.CaptureSlicePixelWidth 720")
    ;[1 1 1] And then for 4096x4096 captures (4096*2048 per eye)
    ;
    ; SP.StepCaptureWidth 4096
    ;
    ; Or for 6144x6144 captures
    ;
    ; SP.StepCaptureWidth 6144
    (`KismetSystemLibrary.ExecuteConsoleCommand` "SP.StepCaptureWidth 4096")
    ;[1 1 1] Export Frame
    (`KismetSystemLibrary.ExecuteConsoleCommand` "SP.PanoramicScreenshot")))

(fn `UserConstructionScript`)