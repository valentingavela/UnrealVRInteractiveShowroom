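; BtnInteractivo is an interactive button actor that changes its static mesh's material when the player presses F nearby.
; Box overlap enables and disables input, and entering also hides the PresionaF prompt, which is never shown again here.
; A looping MultiGate cycles the material between transparent and MATCapa1, with the latter assigned to two of three steps.
; Tick rotates the prompt along the camera-to-text direction as a billboard.
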(event `self.Box.OnComponentBeginOverlap`
  (params (OverlappedComponent :type "PrimitiveComponent Object Reference") (OtherActor :type "Actor Object Reference") (OtherComp :type "PrimitiveComponent Object Reference") (OtherBodyIndex :type Integer) (bFromSweep :type Boolean) (SweepResult :type "HitResult Structure (by ref)"))
  ;[1 1 1] Widget Contrls
  (`self.EnableInput` (`GameplayStatics.GetPlayerController` 0))
  (`SceneComponent.SetVisibility` (`self.Presiona F`) false false))

(event `self.Box.OnComponentEndOverlap`
  (params (OverlappedComponent :type "PrimitiveComponent Object Reference") (OtherActor :type "Actor Object Reference") (OtherComp :type "PrimitiveComponent Object Reference") (OtherBodyIndex :type Integer))
  ;[1 1 1] Widget Contrls
  (`self.DisableInput` (`GameplayStatics.GetPlayerController` 0)))

(event `Key|F`
  (params (Key :type "Key Structure"))
  (bind _staticmesh (`self.StaticMesh`))
  ;[1 1 1] Change Textures
  (:`Pressed`
    (`|MultiGate` false true
      (:`Out 0`
        (`PrimitiveComponent.SetMaterial` _staticmesh 0 "/Game/Materials/old/MATTransparente.MATTransparente"))
      (:`Out 1`
        (`PrimitiveComponent.SetMaterial` _staticmesh 0 "/Game/Materials/old/MATCapa1.MATCapa1"))
      (:`Out 2`
        (`PrimitiveComponent.SetMaterial` _staticmesh 0 "/Game/Materials/old/MATCapa1.MATCapa1")))))

(event `self.ReceiveTick`
  (params (DeltaSeconds :type "Float (single-precision)"))
  ;[1 1 1] Text look Pawn ever
  (`SceneComponent.K2_SetWorldRotation` (`self.Presiona F`) (`KismetMathLibrary.MakeRotFromX` (- (`SceneComponent.K2_GetComponentLocation` (`self.Presiona F`)) (`self.K2_GetActorLocation` (`GameplayStatics.GetPlayerCameraManager` 0)))) false false))

(fn `UserConstructionScript`)