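; Imported FBX scene actor (L200) that moves itself toward a target location, labeled as near the player, when the motion controller's right trigger is pressed.
; Box overlaps and the OnBlur/OnDeblur events toggle player input on the actor.
; The blur events also show or hide a press-trigger prompt and set status text.
; A timeline lerps from the current location to ACTORBP each update, so the start point shifts as it moves.
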(event `self.Box.OnComponentBeginOverlap`
  (params (OverlappedComponent :type "PrimitiveComponent Object Reference") (OtherActor :type "Actor Object Reference") (OtherComp :type "PrimitiveComponent Object Reference") (OtherBodyIndex :type Integer) (bFromSweep :type Boolean) (SweepResult :type "HitResult Structure (by ref)"))
  ;[1 1 1] Widget Contrls
  (`self.EnableInput` (`GameplayStatics.GetPlayerController` 0)))

(event `self.Box.OnComponentEndOverlap`
  (params (OverlappedComponent :type "PrimitiveComponent Object Reference") (OtherActor :type "Actor Object Reference") (OtherComp :type "PrimitiveComponent Object Reference") (OtherBodyIndex :type Integer))
  ;[1 1 1] Widget Contrls
  (`self.DisableInput` (`GameplayStatics.GetPlayerController` 0)))

(event `/Game/Blueprints/Btn1_Interface_BP.OnBlur`
  ;[1 1 1] Widget Contrls
  (`self.EnableInput` (`GameplayStatics.GetPlayerController` 0))
  (`SceneComponent.SetVisibility` (`self.PresionaTrigger`) true false)
  (`TextRenderComponent.K2_SetText` (`self.TextRender`) (`self.Blur`)))

(event `/Game/Blueprints/Btn1_Interface_BP.OnDeblur`
  ;[1 1 1] Widget Contrls
  (`self.DisableInput` (`GameplayStatics.GetPlayerController` 0))
  (`SceneComponent.SetVisibility` (`self.PresionaTrigger`) false false)
  (`TextRenderComponent.K2_SetText` (`self.TextRender`) (`self.Deblur`)))

(event `Key|MotionController_Right_Trigger`
  (params (Key :type "Key Structure"))
  ;[1 1 1] Translate near player
  (:`Pressed`
    (bind (_direction _newtrack_0) (`Timeline|Timeline_0`)
      (:`Update`
        (`self.K2_SetActorLocation` (`KismetMathLibrary.VLerp` (`self.K2_GetActorLocation`) (`self.ACTORBP`) _newtrack_0))))))

(fn `UserConstructionScript`)